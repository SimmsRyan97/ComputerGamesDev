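; Moving spike hazard that costs the player a hit and sends them back to a fixed position.
; On BeginPlay a timeline moves the root, adding its vector track to the spike's starting world location.
; Any actor overlap teleports the player character and calls Hit on ThirdPersonGameMode, without checking which actor overlapped.
; Tick polls the Collected flag in the GlobalVariables game instance and destroys the spike once it is set.
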(event EventBeginPlay
  ;[1 1 1] Moving Spikes
  (bind _output_get (Variables|Default|SetLocation (Transformation|GetWorldLocation (Variables|Default|GetSpike))))
  (bind _newtrack_1 (Timeline|Timeline_0 Play)
    (:Update
      (Transformation|SetWorldLocation (Variables|Default|GetDefaultSceneRoot) (+ _newtrack_1 _output_get) false false))))

(event EventTick
  (params (DeltaSeconds :type Float%20%28single-precision%29))
  ;[1 1 1] When Collected, Remove Spike
  (bind _asglobal_variables (Utilities|Casting|CastToGlobalVariables (Game|GetGameInstance)))
  (if (Variables|/Game/Blueprints/GlobalVariables.GlobalVariables_C|GetCollected _asglobal_variables)
    (Actor|DestroyActor)))

(event Collision|EventActorBeginOverlap
  (params (OtherActor :type Actor%20Object%20Reference))
  ;[1 1 1] If Hit, Take Health and Move Player
  (bind _asnew_character (Utilities|Casting|CastToNewCharacter (Game|GetPlayerCharacter 0)))
  (Transformation|SetWorldLocation (Variables|/Script/Engine.Actor|GetRootComponent _asnew_character) "-1390.000000,220.000000,1080.000000" false false)
  (bind _asthird_person_game_mode (Utilities|Casting|CastToThirdPersonGameMode (Game|GetGameMode)))
  (Default|Hit _asthird_person_game_mode))

(fn ConstructionScript)