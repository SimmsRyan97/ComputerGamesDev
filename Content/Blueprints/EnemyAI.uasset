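; EnemyAI is the zombie enemy's AI logic, which starts pursuit behavior once the game instance's Collected flag is set.
; Tick polls that flag on GlobalVariables and, while it is true, calls ZombieRun through a two-second Delay, so the call recurs.
; ZombieRun sets up the Enemy blackboard, stores the player character in its Player key and runs the Move behavior tree.
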(event EventTick
  (params (DeltaSeconds :type Float%20%28single-precision%29))
  ;[1 1 1] Enemy AI Movement
  (bind _asglobal_variables (Utilities|Casting|CastToGlobalVariables (Game|GetGameInstance)))
  (if (Variables|/Game/Blueprints/GlobalVariables.GlobalVariables_C|GetCollected _asglobal_variables)
    (Utilities|FlowControl|Delay 2.0)
    (CallFunction|ZombieRun)))

(fn ConstructionScript)

(fn ZombieRun
  ;[1 1 1] Adds Blackboard and Behaviour Tree
  (bind _blackboardcomponent (Class|AIController|UseBlackboard "/Game/Blueprints/Enemy.Enemy"))
  (AI|Components|Blackboard|SetValueasObject _blackboardcomponent (Variables|Default|GetPlayer) (Game|GetPlayerCharacter 0))
  (AI|RunBehaviorTree "/Game/Blueprints/Move.Move"))