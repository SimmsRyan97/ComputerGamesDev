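; FloorReset is an overlap-triggered reset floor that sends the player back and takes health.
; On overlap, MovePlayer teleports a NewCharacter to a hard-coded location and sets the Human flag in the GlobalVariables game instance.
; When that flag is set, the event calls Hit on ThirdPersonGameMode, clears the flag and plays the Ouch sound at world origin.
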(event Collision|EventActorBeginOverlap
  (params (OtherActor :type Actor%20Object%20Reference))
  ;[1 1 1] Resets Player and Takes Health
  (CallFunction|MovePlayer OtherActor)
  (bind _asglobal_variables (Utilities|Casting|CastToGlobalVariables (Game|GetGameInstance)))
  (if (Variables|/Game/Blueprints/GlobalVariables.GlobalVariables_C|GetHuman _asglobal_variables)
    (bind _asthird_person_game_mode (Utilities|Casting|CastToThirdPersonGameMode (Game|GetGameMode)))
    (Default|Hit _asthird_person_game_mode)
    (bind _asglobal_variables_2 (Utilities|Casting|CastToGlobalVariables (Game|GetGameInstance)))
    (Variables|/Game/Blueprints/GlobalVariables.GlobalVariables_C|SetHuman _asglobal_variables_2 false)
    (Audio|PlaySoundatLocation "/Game/Sound/Ouch.Ouch" "0, 0, 0")))

(fn ConstructionScript)

(fn MovePlayer
  (params (Actor :type Actor%20Object%20Reference))
  ;[1 1 1] Moves Player Back to Location
  (bind _asnew_character (Utilities|Casting|CastToNewCharacter Actor))
  (Transformation|SetWorldLocation (Variables|/Script/Engine.Actor|GetRootComponent _asnew_character) "-3620.000000,135.000000,900.000000" false false)
  (bind _asglobal_variables (Utilities|Casting|CastToGlobalVariables (Game|GetGameInstance)))
  (Variables|/Game/Blueprints/GlobalVariables.GlobalVariables_C|SetHuman _asglobal_variables true))