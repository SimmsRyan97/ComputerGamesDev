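; Collectible diamond actor that the player picks up with the E key.
; Overlap with NewCharacter enables input on the actor for player controller 0, and ending the overlap disables it.
; Pressing E destroys the actor, then sets the Collected flag on the GlobalVariables game instance.
; A yaw spin for the diamond mesh exists but is disconnected from Tick, so it never runs.
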(event Collision|EventActorBeginOverlap
  (params (OtherActor :type Actor%20Object%20Reference))
  ;[1 1 1] Enables / Disables Keyboard
  (Utilities|Casting|CastToNewCharacter OtherActor)
  (Input|EnableInput (Game|GetPlayerController 0)))

(event EventTick
  (params (DeltaSeconds :type Float%20%28single-precision%29))
  ;[1 1 1] Rotate Diamond
)

(event Collision|EventActorEndOverlap
  (params (OtherActor :type Actor%20Object%20Reference))
  ;[1 1 1] Enables / Disables Keyboard
  (Utilities|Casting|CastToNewCharacter OtherActor)
  (Input|DisableInput (Game|GetPlayerController 0)))

(event Input|KeyboardEvents|E
  (params (Key :type Key%20Structure))
  ;[1 1 1] Press E to Pickup
  (:Pressed
    (Actor|DestroyActor)
    (bind _asglobal_variables (Utilities|Casting|CastToGlobalVariables (Game|GetGameInstance)))
    (Variables|/Game/Blueprints/GlobalVariables.GlobalVariables_C|SetCollected _asglobal_variables true)))

(fn ConstructionScript)